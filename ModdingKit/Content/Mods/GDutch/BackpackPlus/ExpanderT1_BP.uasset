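; Tier 1 backpack expander item that provides four extra item slots while it sits in an auxiliary slot.
; Placement in an aux slot shows the meshes, enables the slots and orients for left or right by mirroring the pipe and shifting the slot mesh.
; Release or other placement force-ejects held items, then hides and disables everything.
; BeginPlay reapplies visibility and slot state from IsInAux, but not the side orientation.
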(event `self.ReceiveBeginPlay`
  (if (`self.IsInAux`)
    (`self.Show`)
    (else
      (`self.Hide`))))

(event `self.PlacedInSlot`
  (params (Slot :type "SlotReference Structure") (FromTool :type Boolean) (SlottedDuringInitialization :type Boolean))
  (if (`SlotStatics.IsSlotAnAuxSlot` Slot)
    (`self.Show`)
    (set `self.IsInAux` true)
    (if (`|EnumEquality` (`SlotStatics.GetAuxSlotType` Slot) "Left")
      (`self.Left`)
      (else
        (`self.Right`)))
    (else
      (`self.Hide`)
      (set `self.IsInAux` false))))

(event `self.ReleasedFromSlot`
  (params (FromTool :type Boolean) (NewOwner :type Boolean))
  (`self.Hide`)
  (set `self.IsInAux` false))

(fn `GetBodySlotLegacy`
  (returns (ReturnValue :type "ChildSlotComponent Object Reference"))
  (return (`self.BodySlot1`)))

(fn `Hide`
  (bind _returnvalue (`ChildSlotComponent.MakeReference` (`self.Slot3`)))
  (bind _returnvalue_2 (`ChildSlotComponent.MakeReference` (`self.Slot2`)))
  (bind _returnvalue_3 (`ChildSlotComponent.MakeReference` (`self.Slot1`)))
  (bind _returnvalue_4 (`ChildSlotComponent.MakeReference` (`self.Slot3`)))
  (bind _returnvalue_5 (`ChildSlotComponent.MakeReference` (`self.Slot4`)))
  (bind _returnvalue_6 (`ChildSlotComponent.MakeReference` (`self.Slot2`)))
  (bind _returnvalue_7 (`ChildSlotComponent.MakeReference` (`self.Slot4`)))
  (bind _returnvalue_8 (`ChildSlotComponent.MakeReference` (`self.Slot1`)))
  (`|ExecutionSequence`
    (:`then_0`
      (if (`SlotStatics.HasAnyItem` _returnvalue_8)
        (`SlotsComponent.ReleaseSlotItemForce` _returnvalue_8)))
    (:`then_1`
      (if (`SlotStatics.HasAnyItem` _returnvalue_6)
        (`SlotsComponent.ReleaseSlotItemForce` _returnvalue_6)))
    (:`then_2`
      (if (`SlotStatics.HasAnyItem` _returnvalue_4)
        (`SlotsComponent.ReleaseSlotItemForce` _returnvalue_4)))
    (:`then_3`
      (if (`SlotStatics.HasAnyItem` _returnvalue_7)
        (`SlotsComponent.ReleaseSlotItemForce` _returnvalue_7)))
    (:`then_4`
      (`SceneComponent.SetVisibility` (`self.PipeMesh`) false false)
      (`SceneComponent.SetVisibility` (`self.SlotsMesh`) false false)
      (`SlotsComponent.SlotEnable` _returnvalue_3)
      (`SlotsComponent.SetSlotAcceptsItems` _returnvalue_3)
      (`SlotsComponent.SlotEnable` _returnvalue_2)
      (`SlotsComponent.SetSlotAcceptsItems` _returnvalue_2)
      (`SlotsComponent.SlotEnable` _returnvalue)
      (`SlotsComponent.SetSlotAcceptsItems` _returnvalue)
      (`SlotsComponent.SlotEnable` _returnvalue_5)
      (`SlotsComponent.SetSlotAcceptsItems` _returnvalue_5))))

(fn `Left`
  (`SceneComponent.SetRelativeScale3D` (`self.PipeMesh`) (1.0 1.0 1.0))
  (`SceneComponent.K2_SetRelativeLocation` (`self.SlotsMesh`) (0.0 0.0 0.0) false false))

(fn `Right`
  (`SceneComponent.SetRelativeScale3D` (`self.PipeMesh`) (-1.0 1.0 1.0))
  (`SceneComponent.K2_SetRelativeLocation` (`self.SlotsMesh`) (-96.0 0.0 0.0) false false))

(fn `Show`
  (bind _returnvalue (`ChildSlotComponent.MakeReference` (`self.Slot3`)))
  (bind _returnvalue_2 (`ChildSlotComponent.MakeReference` (`self.Slot2`)))
  (bind _returnvalue_3 (`ChildSlotComponent.MakeReference` (`self.Slot4`)))
  (bind _returnvalue_4 (`ChildSlotComponent.MakeReference` (`self.Slot1`)))
  (`SceneComponent.SetVisibility` (`self.PipeMesh`) true false)
  (`SceneComponent.SetVisibility` (`self.SlotsMesh`) true false)
  (`SlotsComponent.SlotEnable` _returnvalue_4 true)
  (`SlotsComponent.SetSlotAcceptsItems` _returnvalue_4 true)
  (`SlotsComponent.SlotEnable` _returnvalue_2 true)
  (`SlotsComponent.SetSlotAcceptsItems` _returnvalue_2 true)
  (`SlotsComponent.SlotEnable` _returnvalue true)
  (`SlotsComponent.SetSlotAcceptsItems` _returnvalue true)
  (`SlotsComponent.SlotEnable` _returnvalue_3 true)
  (`SlotsComponent.SetSlotAcceptsItems` _returnvalue_3 true))

(fn `UserConstructionScript`)