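; STORAGEX network node that moves resources between its ResourceSlot and a Storage_BP actor shared by matching SXID.
; Each enabled tick, exporters withdraw the selected type into an empty slot and gradually fill the item.
; Importers empty the slot into storage, subject to count and type limits, spawning the storage actor if none matches.
; BeginPlay and OnRep handlers refresh the child control panel's settings text.
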(event `self.ReceiveTick`
  (params (DeltaSeconds :type "Float (single-precision)"))
  (bind _selected (`self.Selected`))
  (bind _returnvalue (`SlotsComponent.MakeReference` (`self.SlotsComponent`) "ResourceSlot"))
  (bind _returnvalue_2 (`SlotsComponent.GetSlotPrimaryItem` (`SlotsComponent.MakeReference` (`self.SlotsComponent`) "ResourceSlot")))
  (bind _returnvalue_3 (`self.GetComponentByClass` _returnvalue_2 "/Script/Astro.ItemComponent"))
  (bind _itemcomponent (`PhysicalItem.ItemComponent` (`SlotsComponent.GetSlotItem` _returnvalue)))
  (bind _itemtype (`ItemComponent.ItemType` _returnvalue_3))
  (if (`self.IsEnabled`)
    (if (`self.IsExporter`)
      (if (!= (`self.Selected`) null)
        (if (not (`SlotStatics.HasAnyItem` (`SlotsComponent.MakeReference` (`self.SlotsComponent`) "ResourceSlot")))
          (bind (_found _storageactor) (`self.FindStorageWithID`))
          (if _found
            (bind _asstorage_bp (cast `/Game/Mods/GDutch/STORAGEX/Storage_BP` _storageactor))
            (bind _output_get (set `self.StorageActor` _asstorage_bp))
            (bind (_value _returnvalue_4) (`BlueprintMapLibrary.Map_Find` (`/Game/Mods/GDutch/STORAGEX/Storage_BP.Storage` _output_get) (`self.Selected`)))
            (if _returnvalue_4
              (if (>= _value 1)
                (`/Game/Mods/GDutch/STORAGEX/Storage_BP.UpdateStorage` (`self.StorageActor`) _selected -1)
                (`SlotsComponent.SpawnItemTypeInSlot` _returnvalue _selected)
                (`ItemComponent.AddItemRate` _itemcomponent _selected 3.0 :!label _label)
                (if (not (`ItemComponent.IsFull` _itemcomponent))
                  (`KismetSystemLibrary.Delay` 0.01)
                  (goto _label)))))))
      (else
        (`/Engine/EditorBlueprintResources/StandardMacros.IsValid` _returnvalue_2
          (:`Is Valid`
            (bind (_found_2 _storageactor_2) (`self.FindStorageWithID`))
            (if _found_2
              (bind _asstorage_bp_2 (cast `/Game/Mods/GDutch/STORAGEX/Storage_BP` _storageactor_2))
              (bind _output_get_2 (set `self.StorageActor` _asstorage_bp_2))
              (bind _storage (`/Game/Mods/GDutch/STORAGEX/Storage_BP.Storage` _output_get_2))
              (bind (_value_2 _returnvalue_5) (`BlueprintMapLibrary.Map_Find` _storage _itemtype))
              (if _returnvalue_5
                (if (< _value_2 4000)
                  (`/Game/Mods/GDutch/STORAGEX/Storage_BP.UpdateStorage` (`self.StorageActor`) _itemtype 1 :!label _label_2)
                  (`SlotStatics.TakeItem` (`SlotsComponent.MakeReference` (`self.SlotsComponent`) "ResourceSlot") _itemtype (`ItemComponent.Amount` _returnvalue_3)))
                (elif (<= (`BlueprintMapLibrary.Map_Length` _storage) 5)
                  (goto _label_2)))
              (else
                (bind _returnvalue_6 (`|SpawnActorFromClass` "/Game/Mods/GDutch/STORAGEX/Storage_BP.Storage_BP_C" (`KismetMathLibrary.MakeTransform` (0.0 0.0 0.0)) "AlwaysSpawn" "OverrideRootScale" null null))
                (set `/Game/Mods/GDutch/STORAGEX/Storage_BP.SXID` (`self.SXID`) _returnvalue_6)
                (set `self.StorageActor` _returnvalue_6)
                (goto _label_2)))))))))

(event `self.ReceiveBeginPlay`
  (`self.UpdateThisNode`))

(fn `FindStorageWithID`
  (returns (Found :type Boolean) (StorageActor :type "Actor Object Reference"))
  (bind _outactors (`GameplayStatics.GetAllActorsOfClass` "/Game/Mods/GDutch/STORAGEX/Storage_BP.Storage_BP_C"))
  (for _array_element _outactors
    (bind _asstorage_bp (cast `/Game/Mods/GDutch/STORAGEX/Storage_BP` _array_element))
    (if (== (`/Game/Mods/GDutch/STORAGEX/Storage_BP.SXID` _asstorage_bp) (`self.SXID`))
      (return true _array_element)))
  (return false null))

(fn `GetBodySlotLegacy`
  (returns (ReturnValue :type "ChildSlotComponent Object Reference"))
  (return (`self.BodySlot`)))

(fn `OnRep_IsEnabled`
  (`self.UpdateSettingsText`))

(fn `OnRep_IsExporter`
  (`self.UpdateSettingsText`))

(fn `OnRep_Selected`
  (`self.UpdateSettingsText`))

(fn `OnRep_SXID`
  (`self.UpdateSettingsText`))

(fn `UpdateSettingsText`
  (bind _asstoragexcontrol_panel (cast `/Game/Mods/GDutch/STORAGEX/STORAGEXControlPanel` (`ChildActorComponent.ChildActor` (`self.ChildActor`))))
  (`/Game/Mods/GDutch/STORAGEX/STORAGEXControlPanel.UpdateText1` _asstoragexcontrol_panel (`self.SXID`) (`self.IsEnabled`) (`self.IsExporter`) (`self.Selected`)))

(fn `UpdateThisNode`
  (`self.UpdateSettingsText`))

(fn `UserConstructionScript`)