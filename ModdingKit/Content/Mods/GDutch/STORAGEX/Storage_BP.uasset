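; Storage_BP is a Blueprint that holds an item storage map for the STORAGEX mod, tracking an amount for each item type.
; UpdateStorage adds a signed amount to the current count, treating missing types as zero, and removes the entry when the total drops below one.
; A node-refresh call keyed by SXID is left disconnected, noted as not needed until a resource list exists.
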(event `self.ReceiveBeginPlay`)

(fn `UpdateStorage`
  (params (ItemType :type "ItemType Class Reference") (AmountToAdd :type Integer))
  (locals (OldAmount :type Integer))
  (bind _storage (`self.Storage`))
  (bind (_value _returnvalue) (`BlueprintMapLibrary.Map_Find` _storage ItemType))
  (bind _output_get (set `local.OldAmount` (select `bool` _returnvalue :`true` _value)))
  (bind _returnvalue_2 (+ _output_get AmountToAdd))
  (if (< _returnvalue_2 1)
    (`BlueprintMapLibrary.Map_Remove` _storage ItemType)
    (else
      (`BlueprintMapLibrary.Map_Add` _storage ItemType _returnvalue_2))))

(fn `UserConstructionScript`)