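; PLANETX_BP is a mod Blueprint that gives the local player on the server a toggleable PLANETX menu.
; On BeginPlay, if running as server, it creates the MENU_PLANETX widget, adds it to the viewport hidden and enables input for the local player controller.
; Ctrl+N, also gated by a server check, flips the widget between visible and hidden.
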(event `self.ReceiveBeginPlay`
  (bind _returnvalue (`AstroPlayStatics.GetLocalPlayController`))
  (if (`AstroStatics.IsServer`)
    (bind _returnvalue_2 (`|CreateWidget` "/Game/Mods/GDutch/PLANETX/MENU_PLANETX.MENU_PLANETX_C" _returnvalue))
    (`UserWidget.AddToViewport` _returnvalue_2 0)
    (`Widget.SetVisibility` _returnvalue_2 "Hidden")
    (`self.EnableInput` _returnvalue)))

(event `Key|Ctrl+N` :consume false :overrideparent false
  (params (Key :type "Key Structure"))
  (:`Pressed`
    (if (`AstroStatics.IsServer`)
      (`Widget.SetVisibility` (stale `self.ReceiveBeginPlay` _returnvalue_2) (select `ESlateVisibility` (`Widget.GetVisibility` (stale `self.ReceiveBeginPlay` _returnvalue_2)) :`Visible` "Hidden" :`Collapsed` "Visible" :`Hidden` "Visible" :`HitTestInvisible` "Visible" :`SelfHitTestInvisible` "Visible" :!type "ESlateVisibility Enum")))))

(fn `UserConstructionScript`)