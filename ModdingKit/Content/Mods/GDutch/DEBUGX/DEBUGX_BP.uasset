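; DEBUGX mod actor that gives the host a toggleable debug menu.
; On begin play it deletes unused saves, then on the server creates its save object, shows a splash with the shortcut hint and adds the hidden menu widget.
; Ctrl+B toggles the menu's visibility on the server.
; Non-hosts get a "not the host" error splash, both on begin play and on each Ctrl+B press.
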(event `self.ReceiveBeginPlay`
  (bind _returnvalue (`AstroPlayStatics.GetLocalPlayController`))
  (bind _returnvalue_2 (`AstroPlayStatics.GetLocalPlayController`))
  (`/Game/Mods/GDutch/DEBUGX/FUNCS_DEBUGX.DeleteUnusedSaves`)
  (if (`AstroStatics.IsServer`)
    (bind _returnvalue_3 (`GameplayStatics.CreateSaveGameObject` "/Game/Mods/GDutch/DEBUGX/SAVE_DEBUGX.SAVE_DEBUGX_C"))
    (set `self.SaveObj` _returnvalue_3)
    (bind _returnvalue_4 (`|CreateWidget` "/Game/Mods/GDutch/DEBUGX/SPLASH_DEBUGX.SPLASH_DEBUGX_C" _returnvalue_2 "DEBUGX ACTIVE" "PRESS CTRL+B TO OPEN"))
    (`UserWidget.AddToViewport` _returnvalue_4 0)
    (`Widget.SetVisibility` _returnvalue_4 "Visible")
    (`Widget.SetRenderTranslation` _returnvalue_4 (15.0 950.0))
    (bind _returnvalue_5 (`|CreateWidget` "/Game/Mods/GDutch/DEBUGX/MENU_DEBUGX.MENU_DEBUGX_C" _returnvalue_2))
    (`UserWidget.AddToViewport` _returnvalue_5 0)
    (`Widget.SetVisibility` _returnvalue_5 "Hidden")
    (`self.EnableInput` _returnvalue_2)
    (else
      (bind _returnvalue_6 (`|CreateWidget` "/Game/Mods/GDutch/DEBUGX/SPLASH_DEBUGX.SPLASH_DEBUGX_C" _returnvalue "DEBUGX ERROR" "YOU ARE NOT THE HOST" 0.0))
      (`UserWidget.AddToViewport` _returnvalue_6 0)
      (`Widget.SetVisibility` _returnvalue_6 "Visible")
      (`Widget.SetRenderTranslation` _returnvalue_6 (15.0 950.0))
      (`self.EnableInput` _returnvalue))))

(event `Key|Ctrl+B` :consume false :overrideparent false
  (params (Key :type "Key Structure"))
  (:`Pressed`
    (if (`AstroStatics.IsServer`)
      (`Widget.SetVisibility` (stale `self.ReceiveBeginPlay` _returnvalue_5) (select `ESlateVisibility` (`Widget.GetVisibility` (stale `self.ReceiveBeginPlay` _returnvalue_5)) :`Visible` "Hidden" :`Collapsed` "Visible" :`Hidden` "Visible" :`HitTestInvisible` "Visible" :`SelfHitTestInvisible` "Visible" :!type "ESlateVisibility Enum"))
      (else
        (bind _returnvalue (`|CreateWidget` "/Game/Mods/GDutch/DEBUGX/SPLASH_DEBUGX.SPLASH_DEBUGX_C" (`AstroPlayStatics.GetLocalPlayController`) "DEBUGX ERROR" "YOU ARE NOT THE HOST" 5.0))
        (`UserWidget.AddToViewport` _returnvalue 0)
        (`Widget.SetVisibility` _returnvalue "Visible")
        (`Widget.SetRenderTranslation` _returnvalue (15.0 950.0))))))

(fn `UserConstructionScript`)